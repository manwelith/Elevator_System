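; Elevator actor that lets the player pick one of four floors from a UI and moves its platform there.
; Interact opens the FloorSelectWP widget once, switching to UI-only input with a visible cursor.
; The floor selection restores game input and sets a fixed height, then plays the Elevator timeline.
; Timeline updates move the Plane toward a lerp from relative origin to that height and re-arm the interaction.
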(event `/Game/Elevator/BPI_Interact.Interact`
  (bind _returnvalue (`GameplayStatics.GetPlayerController` 0))
  (`/Engine/EditorBlueprintResources/StandardMacros.DoOnce` false :!label _label
    (:`Completed`
      (bind _returnvalue_2 (`|CreateWidget` "/Game/Elevator/FloorSelectWP.FloorSelectWP_C"))
      (bind _output_get (set `self.Widget_Ref` _returnvalue_2))
      (`UserWidget.AddToViewport` _output_get 0)
      (`WidgetBlueprintLibrary.SetInputMode_UIOnlyEx` _returnvalue null "LockAlways")
      (set `PlayerController.bShowMouseCursor` true _returnvalue)
      (add `/Game/Elevator/FloorSelectWP.Set_Floor` (`self.Widget_Ref`) (delegate `Event_Floor`)))))

(event `Event_Floor`
  (params (`Clicked?` :type Boolean) (Floor_Selection :type Integer))
  (bind _returnvalue (`GameplayStatics.GetPlayerController` 0))
  (if `Clicked?`
    (`Widget.RemoveFromParent` (`self.Widget_Ref`))
    (`WidgetBlueprintLibrary.SetInputMode_GameOnly` _returnvalue)
    (set `PlayerController.bShowMouseCursor` false _returnvalue)
    (switch `int` Floor_Selection
      (:`1`
        (set `self.Elevator_Floor` (0.0 0.0 0.0))
        (bind (_direction _value) (`Timeline|Elevator` :!label _label_2)
          (:`Update`
            (`KismetSystemLibrary.MoveComponentTo` (`self.Plane`) (`KismetMathLibrary.VLerp` (0.0 0.0 0.0) (`self.Elevator_Floor`) _value) (struct) false false (`self.Elapsed_Time`))
            (goto _label :!via `Reset`))))
      (:`2`
        (set `self.Elevator_Floor` (0.0 0.0 600.0))
        (goto _label_2))
      (:`3`
        (set `self.Elevator_Floor` (0.0 0.0 1200.0))
        (goto _label_2))
      (:`4`
        (set `self.Elevator_Floor` (0.0 0.0 1800.0))
        (goto _label_2)))))

(fn `UserConstructionScript`)